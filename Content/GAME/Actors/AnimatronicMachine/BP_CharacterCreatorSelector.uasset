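; Body-part selector for the animatronic character creator, built from a posed set of part meshes that is presumably viewed through a scene capture.
; A single scene capture is taken on BeginPlay.
; HightlightPart maps a part to its mesh via TypeToMesh and toggles custom depth, with both props sharing the mic mesh.
; SelectPart forwards the chosen part to the BP_CharacterCreator found in the level.
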(event `self.ReceiveBeginPlay`
  (`SceneCaptureComponent2D.CaptureScene` (`self.SceneCaptureComponent2D`)))

(event `/Game/GAME/Actors/AnimatronicMachine/Interfaces/ISelector.HightlightPart`
  (params (Part :type "/Game/GAME/Actors/AnimatronicMachine/Enums/EPartType Enum" :default "NewEnumerator28") (Enabled :type Boolean))
  (`PrimitiveComponent.SetRenderCustomDepth` (`self.TypeToMesh` Part) Enabled))

(event `/Game/GAME/Actors/AnimatronicMachine/Interfaces/ISelector.SelectPart`
  (params (Part :type "/Game/GAME/Actors/AnimatronicMachine/Enums/EPartType Enum" :default "NewEnumerator28"))
  (bind _returnvalue (`GameplayStatics.GetActorOfClass` "/Game/GAME/Actors/AnimatronicMachine/BP_CharacterCreator.BP_CharacterCreator_C"))
  (`/Engine/EditorBlueprintResources/StandardMacros.IsValid` _returnvalue
    (:`Is Valid`
      (`/Game/GAME/Actors/AnimatronicMachine/BP_CharacterCreator.SelectPart` _returnvalue Part))))

(fn `TypeToMesh`
  (params (Index :type "/Game/GAME/Actors/AnimatronicMachine/Enums/EPartType Enum" :default "NewEnumerator0"))
  (returns (ReturnValue :type "PrimitiveComponent Object Reference"))
  (bind _creator_pose_mic (`self.Creator_Pose_Mic`))
  (return (select `/Game/GAME/Actors/AnimatronicMachine/Enums/EPartType` Index :`NewEnumerator0` (`self.Creator_Pose_Mask`) :`NewEnumerator1` (`self.Creator_Pose_Torso`) :`NewEnumerator2` (`self.Creator_Pose_Bowtie`) :`NewEnumerator3` (`self.Creator_Pose_Hat`) :`NewEnumerator4` (`self.Creator_Pose_Jaw`) :`NewEnumerator5` (`self.Creator_Pose_Pelvis`) :`NewEnumerator6` (`self.Creator_Pose_UpperArm_R`) :`NewEnumerator7` (`self.Creator_Pose_UpperArm_L`) :`NewEnumerator8` (`self.Creator_Pose_LowerArm_R`) :`NewEnumerator9` (`self.Creator_Pose_LowerArm_L`) :`NewEnumerator10` (`self.Creator_Pose_Hand_R`) :`NewEnumerator11` (`self.Creator_Pose_Hand_L`) :`NewEnumerator12` (`self.Creator_Pose_UpperLeg_R`) :`NewEnumerator13` (`self.Creator_Pose_UpperLeg_L`) :`NewEnumerator14` (`self.Creator_Pose_LowerLeg_R`) :`NewEnumerator15` (`self.Creator_Pose_LowerLeg_L`) :`NewEnumerator16` (`self.Creator_Pose_Foot_R`) :`NewEnumerator17` (`self.Creator_Pose_Foot_L`) :`NewEnumerator18` (`self.Creator_Pose_Knee_R`) :`NewEnumerator19` (`self.Creator_Pose_Knee_L`) :`NewEnumerator20` (`self.Creator_Pose_Shoulder_R`) :`NewEnumerator21` (`self.Creator_Pose_Shoulder_L`) :`NewEnumerator22` (`self.Creator_Pose_Ear_R`) :`NewEnumerator23` (`self.Creator_Pose_Ear_L`) :`NewEnumerator26` _creator_pose_mic :`NewEnumerator27` _creator_pose_mic :!type "PrimitiveComponent Object Reference")))

(fn `UserConstructionScript`)