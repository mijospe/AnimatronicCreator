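; BP_Camera is a camera actor that becomes the player's view target on BeginPlay and takes input to orbit its spring arm.
; Mouse2D input, scaled by CameraSpeed, adds pitch and yaw to the SpringArm without checking the right mouse button.
; Holding that button hides the cursor and runs a fast looping timer, apparently driving OnCameraUpdate to re-center the mouse.
; Release restores the cursor and clears the timer; MoveCamera is an empty stub.
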(event `self.ReceiveBeginPlay`
  (`PlayerController.SetViewTargetWithBlend` (`GameplayStatics.GetPlayerController` 0) self 0.0 "VTBlend_Linear" 0.0 false)
  (`self.EnableInput` (`GameplayStatics.GetPlayerController` 0)))

(event `Key|RightMouseButton`
  (params (Key :type "Key Structure"))
  (:`Pressed`
    (set `PlayerController.bShowMouseCursor` false (`GameplayStatics.GetPlayerController` 0))
    (bind _returnvalue (`KismetSystemLibrary.K2_SetTimerDelegate` (`|CreateDelegate` :!event `OnCameraUpdate`) 0.0001 true true))
    (set `self.Timer_UpdateCamera` _returnvalue))
  (:`Released`
    (set `PlayerController.bShowMouseCursor` true (`GameplayStatics.GetPlayerController` 0))
    (`KismetSystemLibrary.K2_ClearAndInvalidateTimerHandle` (`self.Timer_UpdateCamera`))))

(event `InputVectorAxis|Mouse2D`
  (params (AxisValue :type "Vector Structure"))
  (bind (_returnvalue_x _returnvalue_y) (`KismetMathLibrary.BreakVector` (* AxisValue (`self.CameraSpeed`))))
  (`SceneComponent.K2_AddRelativeRotation` (`self.SpringArm`) (`KismetMathLibrary.MakeRotator` 0.0 _returnvalue_y _returnvalue_x) false false))

(event `self.ReceiveTick`
  (params (DeltaSeconds :type "Float (single-precision)")))

(event `OnCameraUpdate`
  (bind (_returnvalue_x _returnvalue_y) (`KismetMathLibrary.BreakVector2D` (`WidgetLayoutLibrary.GetViewportSize`)))
  (`PlayerController.SetMouseLocation` (`GameplayStatics.GetPlayerController` 0) (`KismetMathLibrary.FTrunc` (* _returnvalue_x 0.5)) (`KismetMathLibrary.FTrunc` (* _returnvalue_y 0.5))))

(fn `MoveCamera`)

(fn `UserConstructionScript`)